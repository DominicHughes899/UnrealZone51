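; Prototype falling-obstacle actor that telegraphs a spinning cylinder drop, then destroys itself after a fixed lifetime.
; Tick ramps a dynamic fading-red material on the warning plane until Delay, then hides the warning visuals and starts the fall.
; AnimateCylinder rotates and moves the cylinder every frame, zeroing fall speed at a hard-coded world height.
; Actor overlaps only print debug hurt messages; no damage is applied.
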(event EventBeginPlay
  (bind _returnvalue (Rendering|Material|CreateDynamicMaterialInstance "/Game/Core/Materials/M_FadingRed.M_FadingRed" "None" "None" :!class /Script/Engine.KismetMaterialLibrary))
  (bind _output_get (Variables|Default|SetMaterialInstance _returnvalue))
  (Rendering|Material|SetMaterial (Variables|Default|GetWarningPlane) 1 _output_get))

(event EventTick
  (params (DeltaSeconds :type Float%20%28single-precision%29))
  (CallFunction|AnimateCylinder DeltaSeconds)
  (bind _output_get (Variables|Default|SetTimer (+ DeltaSeconds (Variables|Default|GetTimer))))
  (Rendering|Material|SetScalarParameterValue (Variables|Default|GetMaterialInstance) "Percent" (Math|Float|Lerp 0.0 1.0 (/ _output_get (Variables|Default|GetDelay))) :!class /Script/Engine.MaterialInstanceDynamic)
  (if (>= _output_get 4.0)
    (Actor|DestroyActor)
    (elif (>= _output_get (Variables|Default|GetDelay))
      (Utilities|FlowControl|DoOnce false
        (:Completed
          (Variables|Default|SetCylinderFallSpeed -5e+03)
          (Rendering|SetVisibility (Variables|Default|GetWarningPlane) false false)
          (Rendering|SetVisibility (Variables|Default|GetSM_WarningTriangle) false false))))))

(event Collision|EventActorBeginOverlap
  (params (OtherActor :type Actor%20Object%20Reference))
  (Development|PrintString "Hurting"))

(event Collision|EventActorEndOverlap
  (params (OtherActor :type Actor%20Object%20Reference))
  (Development|PrintString "not hurting"))

(fn ConstructionScript)

(fn AnimateCylinder
  (params (Dt :type Float%20%28double-precision%29))
  (Transformation|AddLocalRotation (Variables|Default|GetCylinder) (Math|Rotator|MakeRotator 0.0 0.0 (* Dt (LocalVariables|GetRotationRate))) false false)
  (Transformation|AddLocalOffset (Variables|Default|GetCylinder) (Math|Vector|MakeVector 0.0 0.0 (* (Variables|Default|GetCylinderFallSpeed) Dt)) false false)
  (bind _inposition (CallFunction|CheckinPosition))
  (if _inposition
    (Variables|Default|SetCylinderFallSpeed 0.0)))

(fn CheckinPosition
  (return (<= (.z (Transformation|GetWorldLocation (Variables|Default|GetCylinder))) 2.5e+03)))