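; Player character Blueprint for Zone51 that owns the start menu and in-game UI and handles the transition into play.
; BeginPlay creates both widgets with the playing UI hidden, then a DoOnce on Tick pauses the game and focuses the menu's Start widget.
; StartGame unpauses, swaps widget visibility and restores game-only input.
; UpdateUI passes the character's energy level to the playing UI.
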(event EventBeginPlay
  (CallFunction|CreateUI)
  (bind _output_get (Variables|Default|SetPlayerController (Game|GetPlayerController 0)))
  (Variables|/Script/Engine.PlayerController|SetbShowMouseCursor _output_get true))

(event EventTick
  (params (DeltaSeconds :type Float%20%28single-precision%29))
  (Utilities|FlowControl|DoOnce false
    (:Completed
      (Game|SetGamePaused true)
      (Input|SetInputModeUIOnly (Variables|Default|GetPlayerController) (Variables|/Game/Core/UI/WBP_StartMenu.WBP_StartMenu_C|GetStart (Variables|Default|GetStartMenuUI)) "DoNotLock"))))

(event EventUpdateUI
  (bind _returnvalue (Class|CharacterZone51|GetEnergyLevel))
  (Default|UpdateEnergyLevels (Variables|Default|GetMainUI) _returnvalue))

(fn ConstructionScript)

(fn CreateUI
  (bind _returnvalue (UserInterface|CreateWidget "/Game/Core/UI/WBP_StartMenu.WBP_StartMenu_C"))
  (bind _output_get (Variables|Default|SetStartMenuUI _returnvalue))
  (UserInterface|Viewport|AddtoViewport _output_get 0)
  (Variables|/Game/Core/UI/WBP_StartMenu.WBP_StartMenu_C|SetAssociatedCharacter _output_get self)
  (bind _returnvalue_2 (UserInterface|CreateWidget "/Game/Core/UI/WBP_PlayingUI.WBP_PlayingUI_C"))
  (bind _output_get_2 (Variables|Default|SetMainUI _returnvalue_2))
  (UserInterface|Viewport|AddtoViewport _output_get_2 0)
  (Widget|SetVisibility _output_get_2 "Hidden"))

(fn StartGame
  (bind _playercontroller (Variables|Default|GetPlayerController))
  (Game|SetGamePaused false)
  (Widget|SetVisibility (Variables|Default|GetMainUI) "Visible")
  (Widget|SetVisibility (Variables|Default|GetStartMenuUI) "Hidden")
  (Input|SetInputModeGameOnly _playercontroller)
  (Variables|/Script/Engine.PlayerController|SetbShowMouseCursor _playercontroller false))